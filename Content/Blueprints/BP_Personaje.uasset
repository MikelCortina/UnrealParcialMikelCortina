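; BP_Personaje is the player character, with jumping, control-rotation-relative movement and mouse look.
; Overlapping a BP_Moneda coin increments Puntuacion and updates the score through the Interfaz held by GM_Juego, cached on BeginPlay.
; Whenever the score reaches a multiple of ten, it spawns a BP_Enemy at a fixed world location.
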(event Collision|EventActorBeginOverlap
  (params (OtherActor :type Actor%20Object%20Reference))
  (Utilities|Casting|CastToBP_Moneda OtherActor)
  (Math|Integer|IncrementInt (Variables|Default|GetPuntuacion)
    (:%20%20
      (Default|Puntuacion (Variables|/Game/Blueprints/GM_Juego.GM_Juego_C|GetInterfaz (stale EventBeginPlay _asgm_juego)))
      (if (== (Math|Integer|%(Integer) (Variables|Default|GetPuntuacion) 10) 0)
        (Game|SpawnActorfromClass "/Game/Blueprints/BP_Enemy.BP_Enemy_C" (Math|Conversions|ToTransform(Vector) "-520.000000,-210.000000,88.000000") "AdjustIfPossibleButAlwaysSpawn" "MultiplyWithRoot" 0 0)))))

(event EventBeginPlay
  (bind _asgm_juego (Utilities|Casting|CastToGM_Juego (Game|GetGameMode))))

(event Input|ActionEvents|InputActionSaltocubo
  (params (Key :type Key%20Structure :default "None"))
  (:Pressed
    (Character|Jump))
  (:Released
    (Character|StopJumping)))

(event Input|AxisEvents|InputAxisMovimientoadelanteyatras
  (params (AxisValue :type Float%20%28single-precision%29))
  (Pawn|Input|AddMovementInput (Math|Vector|GetForwardVector (Math|Rotator|MakeRotator 0.0 0.0 (.yaw (Pawn|GetControlRotation :!class /Script/Engine.Pawn)))) AxisValue false))

(event Input|AxisEvents|InputAxisMovimientoizquierdayderecha
  (params (AxisValue :type Float%20%28single-precision%29))
  (bind _returnvalue (Pawn|GetControlRotation :!class /Script/Engine.Pawn))
  (Pawn|Input|AddMovementInput (Math|Vector|GetRightVector (Math|Rotator|MakeRotator (.roll _returnvalue) 0.0 (.yaw _returnvalue))) AxisValue false))

(event Input|AxisEvents|InputAxisRatonarribayabajo
  (params (AxisValue :type Float%20%28single-precision%29))
  (Pawn|Input|AddControllerPitchInput AxisValue))

(event Input|AxisEvents|InputAxisRatonizquierdayderecha
  (params (AxisValue :type Float%20%28single-precision%29))
  (Pawn|Input|AddControllerYawInput AxisValue))

(fn ConstructionScript)