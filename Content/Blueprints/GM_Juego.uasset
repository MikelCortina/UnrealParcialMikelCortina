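; Game mode Blueprint, judging by its GM_ name, that sets up the HUD and scatters coins at level start.
; BeginPlay adds the Interfaz widget to the viewport, then SpawnCoins places five BP_Moneda at random BP_Spawnpoint actors, destroying each used point to prevent repeats.
; SpawnRandomCoin, uncalled here, spawns one coin at a random remaining spawn point without consuming it.
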(event EventBeginPlay
  (Utilities|FlowControl|Sequence
    (:then_0
      (bind _returnvalue (UserInterface|CreateWidget "/Game/Interfaz/Interfaz.Interfaz_C"))
      (bind _output_get (Variables|Default|SetInterfaz _returnvalue))
      (UserInterface|Viewport|AddtoViewport _output_get 0))
    (:then_1
      (CallFunction|SpawnCoins))))

(fn ConstructionScript)

(fn SpawnCoins
  (bind _outactors (Actor|GetAllActorsOfClass "/Game/Blueprints/BP_Spawnpoint.BP_Spawnpoint_C"))
  (LocalVariables|SetLocalSpawnPoints _outactors)
  (for _index (range 0 4)
    (LocalVariables|SetLocalItem (.OutItem (Utilities|Array|Random (LocalVariables|GetLocalSpawnPoints))))
    (Game|SpawnActorfromClass "/Game/Blueprints/BP_Moneda.BP_Moneda_C" (Math|Transform|MakeTransform (Transformation|GetActorLocation (LocalVariables|GetLocalItem))) "AdjustIfPossibleButAlwaysSpawn" "MultiplyWithRoot" 0 0)
    (Utilities|Array|RemoveItem (LocalVariables|GetLocalSpawnPoints) (LocalVariables|GetLocalItem))
    (Actor|DestroyActor (LocalVariables|GetLocalItem))))

(fn SpawnRandomCoin
  (bind _outactors (Actor|GetAllActorsOfClass "/Game/Blueprints/BP_Spawnpoint.BP_Spawnpoint_C"))
  (LocalVariables|SetLocalSpawnPoint _outactors)
  (LocalVariables|SetLocalItem (.OutItem (Utilities|Array|Random (LocalVariables|GetLocalSpawnPoint))))
  (Game|SpawnActorfromClass "/Game/Blueprints/BP_Moneda.BP_Moneda_C" (Math|Transform|MakeTransform (Transformation|GetActorLocation (LocalVariables|GetLocalItem))) "AdjustIfPossibleButAlwaysSpawn" "MultiplyWithRoot" 0 0)
  (return))