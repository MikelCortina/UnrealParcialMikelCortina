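; BP_GameManager is an early-stage game manager Blueprint that currently only prints a debug greeting on BeginPlay.
; An unconnected chain would spawn a BP_Moneda coin at a random XY point within the Box component's extent, at the box's height.
; That chain ends in a stray cast to RigVMFunctionReturnNode and never runs.
; The SpawnCoin function and construction script are empty.
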(event EventBeginPlay
  (Development|PrintString "Hello"))

(fn ConstructionScript)

(fn SpawnCoin)